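; Character Blueprint that makes sprites translucent when its BehindObjectChecker component overlaps environment objects, likely to show it is behind them.
; Begin overlap with a BP_Big_Tree's Sprite sets both that sprite and the character's own to partial alpha.
; End overlap accepts any BaseEnvironmentObject and returns both sprites to near-full alpha.
; Both events print a debug "Hello"; the construction script is empty.
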(event OnComponentBeginOverlap(BehindObjectChecker)
  (params (OverlappedComponent :type Primitive%20Component%20Object%20Reference) (OtherActor :type Actor%20Object%20Reference) (OtherComp :type Primitive%20Component%20Object%20Reference) (OtherBodyIndex :type Integer) (bFromSweep :type Boolean) (SweepResult :type Hit%20Result%20Structure%20%28by%20ref%29))
  (bind _asbp_big_tree (Utilities|Casting|CastToBP_Big_Tree OtherActor))
  (if (== OtherComp (Variables|/Script/SimpleGame.BaseObject|GetSprite _asbp_big_tree))
    (Sprite|SetSpriteColor (Variables|Default|GetSprite) "(R=1.000000,G=1.000000,B=1.000000,A=0.700000)")
    (Development|PrintString "Hello")))

(event OnComponentEndOverlap(BehindObjectChecker)
  (params (OverlappedComponent :type Primitive%20Component%20Object%20Reference) (OtherActor :type Actor%20Object%20Reference) (OtherComp :type Primitive%20Component%20Object%20Reference) (OtherBodyIndex :type Integer))
  (bind _asbase_environment_object (Utilities|Casting|CastToBaseEnvironmentObject OtherActor))
  (if (== OtherComp (Variables|/Script/SimpleGame.BaseObject|GetSprite _asbase_environment_object))
    (Sprite|SetSpriteColor (Variables|Default|GetSprite) "(R=1.000000,G=1.000000,B=1.000000,A=0.995000)")
    (Development|PrintString "Hello")))

(fn ConstructionScript)